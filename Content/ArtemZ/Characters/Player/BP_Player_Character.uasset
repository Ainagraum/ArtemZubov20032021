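; Player character handling movement, look, sprint and cooldown-limited jump, plus interaction with lamps and weapons.
; Capsule overlaps track the nearby gun or lamp; interacting toggles the light or attaches the gun, which can fire, alternate-fire or drop with physics.
; StatusAC receives damage and constitution changes from sprinting and jumping.
; On death, the mesh ragdolls with an impulse along the last point-damage direction, movement stops and the weapon drops.
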(event OnComponentBeginOverlap(CapsuleComponent)
  (params (OverlappedComponent :type Primitive%20Component%20Object%20Reference) (OtherActor :type Actor%20Object%20Reference) (OtherComp :type Primitive%20Component%20Object%20Reference) (OtherBodyIndex :type Integer) (bFromSweep :type Boolean) (SweepResult :type Hit%20Result%20Structure%20%28by%20ref%29))
  ;[1 1 1] Overlap
  (Utilities|FlowControl|Sequence
    (:then_0
      (bind _asgun (Utilities|Casting|CastToGun OtherActor))
      (Variables|Default|SetInteractWeapon _asgun))
    (:then_1
      (bind _astest_base_lamp (Utilities|Casting|CastToTestBaseLamp OtherActor))
      (Variables|Default|SetInteractLamp _astest_base_lamp))))

(event OnComponentEndOverlap(CapsuleComponent)
  (params (OverlappedComponent :type Primitive%20Component%20Object%20Reference) (OtherActor :type Actor%20Object%20Reference) (OtherComp :type Primitive%20Component%20Object%20Reference) (OtherBodyIndex :type Integer))
  ;[1 1 1] Overlap
  (Utilities|FlowControl|Sequence
    (:then_0
      (if (== OtherActor (Variables|Default|GetInteractWeapon))
        (Variables|Default|SetInteractWeapon 0)))
    (:then_1
      (if (== OtherActor (Variables|Default|GetInteractLamp))
        (Variables|Default|SetInteractLamp 0)))))

(event OnDeath(StatusAC)
  (Utilities|FlowControl|DoOnce false
    (:Completed
      (Physics|SetSimulatePhysics (Variables|Character|GetMesh) true)
      (Utilities|FlowControl|Delay 0.0)
      (Physics|AddImpulse (Variables|Character|GetMesh) (* (Variables|Default|GetLastPointDamageDirection) 5000) "None" false)
      (Pawn|Components|CharacterMovement|DisableMovement (Variables|Character|GetCharacterMovement))
      (CallFunction|DropWeapon))))

(event EventBeginPlay)

(event Collision|EventActorBeginOverlap
  (params (OtherActor :type Actor%20Object%20Reference)))

(event EventTick
  (params (DeltaSeconds :type Float%20%28single-precision%29))
  ;[1 0.7597 0.7498] Events
  (Utilities|FlowControl|Sequence
    (:then_0
      (if (Variables|Default|GetIsSprinting)
        (Default|ConstitutionLose\Gain (Variables|Default|GetStatusAC) 2.0)
        (else
          (Default|ConstitutionLose\Gain (Variables|Default|GetStatusAC) -0.5))))))

(event Game|Damage|EventAnyDamage
  (params (Damage :type Float%20%28single-precision%29) (DamageType :type Damage%20Type%20Object%20Reference) (InstigatedBy :type Controller%20Object%20Reference) (DamageCauser :type Actor%20Object%20Reference))
  ;[1 0.7597 0.7498] Events
  (Default|MakeDamage\Heal (Variables|Default|GetStatusAC) Damage))

(event Game|Damage|EventPointDamage
  (params (Damage :type Float%20%28single-precision%29) (DamageType :type Damage%20Type%20Object%20Reference) (HitLocation :type Vector :default "0, 0, 0") (HitNormal :type Vector :default "0, 0, 0") (HitComponent :type Primitive%20Component%20Object%20Reference) (BoneName :type Name :default "None") (ShotFromDirection :type Vector :default "0, 0, 0") (InstigatedBy :type Controller%20Object%20Reference) (DamageCauser :type Actor%20Object%20Reference) (HitInfo :type Hit%20Result%20Structure%20%28by%20ref%29))
  ;[1 0.7597 0.7498] Events
  (Variables|Default|SetLastPointDamageDirection ShotFromDirection))

(event Input|ActionEvents|InputActionInteract
  (params (Key :type Key%20Structure :default "None"))
  (bind _interactlamp (Variables|Default|GetInteractLamp))
  ;[0.5718 1 0.9701] Actions
  (:Pressed
    (Utilities|FlowControl|Sequence
      (:then_0
        (if (Utilities|IsValid _interactlamp)
          (Default|SwitchLight _interactlamp (not (Variables|/Game/ArtemZ/Interactions/TestBaseLamp.TestBaseLamp_C|GetOnOff _interactlamp)))))
      (:then_1
        (if (Utilities|IsValid (Variables|Default|GetInteractWeapon))
          (CallFunction|TakeWeapon))))))

(event Input|ActionEvents|InputActionSprint
  (params (Key :type Key%20Structure :default "None"))
  ;[0.5718 1 0.9701] Actions
  (:Pressed
    (Variables|/Script/Engine.CharacterMovementComponent|SetMaxWalkSpeed (Variables|Character|GetCharacterMovement) 9e+02)
    (Variables|Default|SetIsSprinting true))
  (:Released
    (Variables|/Script/Engine.CharacterMovementComponent|SetMaxWalkSpeed (Variables|Character|GetCharacterMovement) 4.5e+02)
    (Variables|Default|SetIsSprinting false)))

(event Input|ActionEvents|InputActionJump
  (params (Key :type Key%20Structure :default "None"))
  ;[0.5718 1 0.9701] Actions
  (:Pressed
    (if (not (Variables|Default|GetJumped))
      (Variables|Default|SetJumped true)
      (Character|Jump)
      (Default|ConstitutionLose\Gain (Variables|Default|GetStatusAC) 2e+01)
      (Utilities|FlowControl|Delay 2.0)
      (Variables|Default|SetJumped false))))

(event Input|ActionEvents|InputActionPrimaryAction
  (params (Key :type Key%20Structure :default "None"))
  (bind _activeweapon (Variables|Default|GetActiveWeapon))
  ;[0.5718 1 0.9701] Actions
  (:Pressed
    (if (Utilities|IsValid _activeweapon)
      (Default|Fire _activeweapon))))

(event Input|ActionEvents|InputActionDropWeapon
  (params (Key :type Key%20Structure :default "None"))
  ;[0.5718 1 0.9701] Actions
  (:Pressed
    (CallFunction|DropWeapon)))

(event Input|ActionEvents|InputActionSecondaryAction
  (params (Key :type Key%20Structure :default "None"))
  (bind _activeweapon (Variables|Default|GetActiveWeapon))
  ;[0.5718 1 0.9701] Actions
  (:Pressed
    (if (Utilities|IsValid _activeweapon)
      (Default|AlternateFire _activeweapon))))

(event Input|AxisEvents|InputAxisMoveForward
  (params (AxisValue :type Float%20%28single-precision%29))
  ;[0.5955 1 0.7673] Movement
  (Pawn|Input|AddMovementInput (Transformation|GetActorForwardVector) AxisValue false))

(event Input|AxisEvents|InputAxisMoveRight
  (params (AxisValue :type Float%20%28single-precision%29))
  ;[0.5955 1 0.7673] Movement
  (Pawn|Input|AddMovementInput (Transformation|GetActorRightVector) AxisValue false))

(event Input|AxisEvents|InputAxisTurn
  (params (AxisValue :type Float%20%28single-precision%29))
  ;[0.5955 1 0.7673] Movement
  (Pawn|Input|AddControllerYawInput AxisValue))

(event Input|AxisEvents|InputAxisLookUp
  (params (AxisValue :type Float%20%28single-precision%29))
  ;[0.5955 1 0.7673] Movement
  (Pawn|Input|AddControllerPitchInput AxisValue))

(event Input|KeyboardEvents|1
  (params (Key :type Key%20Structure :default "None"))
  ;[1 1 1] Animation
  (:Pressed
    (Variables|Default|SetIsCurrentWeapon (not (Variables|Default|GetIsCurrentWeapon)))))

(fn ConstructionScript)

(fn TakeWeapon
  (if (Utilities|IsValid (Variables|Default|GetActiveWeapon))
    (CallFunction|DropWeapon))
  (bind _output_get (Variables|Default|SetActiveWeapon (Variables|Default|GetInteractWeapon)))
  (Transformation|AttachComponentToComponent _output_get (Variables|Default|GetWeaponPlace) "None" "SnapToTarget" "SnapToTarget" "SnapToTarget" true)
  (Collision|SetCollisionEnabled (Variables|/Game/ArtemZ/Weapons/WeaponBaseForWeapons.WeaponBaseForWeapons_C|GetCube (Variables|Default|GetActiveWeapon)) "NoCollision")
  (Physics|SetSimulatePhysics (Variables|/Game/ArtemZ/Weapons/WeaponBaseForWeapons.WeaponBaseForWeapons_C|GetCube (Variables|Default|GetActiveWeapon)) false)
  (Variables|Default|SetInteractWeapon 0))

(fn DropWeapon
  (if (Utilities|IsValid (Variables|Default|GetActiveWeapon))
    (Physics|SetSimulatePhysics (Variables|/Game/ArtemZ/Weapons/WeaponBaseForWeapons.WeaponBaseForWeapons_C|GetCube (Variables|Default|GetActiveWeapon)) true)
    (Collision|SetCollisionEnabled (Variables|/Game/ArtemZ/Weapons/WeaponBaseForWeapons.WeaponBaseForWeapons_C|GetCube (Variables|Default|GetActiveWeapon)) "QueryAndPhysics")
    (Transformation|DetachFromActor (Variables|Default|GetActiveWeapon) "KeepWorld" "KeepWorld" "KeepWorld")
    (Variables|Default|SetActiveWeapon 0)))